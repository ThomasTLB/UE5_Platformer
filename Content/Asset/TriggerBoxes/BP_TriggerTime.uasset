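; BP_TriggerTime is a trigger box that starts a minutes-and-seconds game timer when BP_MyPlayer enters it.
; On overlap, the Start Game Zone Timer zone type sets IsStart and adds a WBP_Timer widget to the viewport.
; While IsStart is set, Tick uses a one-second Delay to increment Seconds, rolling over into Minutes.
; SetTime is an unfinished stub with disconnected conversion nodes.
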(event `self.ReceiveTick`
  (params (DeltaSeconds :type "Float (single-precision)"))
  (if (`self.IsStart`)
    (`KismetSystemLibrary.Delay` 1.0)
    (set `self.Seconds` (+ (`self.Seconds`) 1))
    (if (> (`self.Seconds`) 59)
      (set `self.Minutes` (+ (`self.Minutes`) 1))
      (set `self.Seconds` 0))))

(event `self.Box.OnComponentBeginOverlap`
  (params (OverlappedComponent :type "PrimitiveComponent Object Reference") (OtherActor :type "Actor Object Reference") (OtherComp :type "PrimitiveComponent Object Reference") (OtherBodyIndex :type Integer) (bFromSweep :type Boolean) (SweepResult :type "HitResult Structure (by ref)"))
  (cast `/Game/Asset/Characters/BP_MyPlayer` OtherActor)
  (switch `/Game/Asset/TriggerBoxes/E_TriggerTimer` (`self.ZoneType`)
    (:`NewEnumerator0`
      (set `self.IsStart` true)
      (bind _returnvalue (`|CreateWidget` "/Game/Asset/Widgets/WBP_Timer.WBP_Timer_C"))
      (`UserWidget.AddToViewport` _returnvalue 0))))

(fn `SetTime`
  (params (Qt :type Integer))
  (`|ExecutionSequence`))

(fn `UserConstructionScript`)