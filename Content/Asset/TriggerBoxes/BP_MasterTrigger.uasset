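; BP_MasterTrigger is a multipurpose trigger box that acts as a death, checkpoint or win zone, chosen by its ZoneType.
; On overlap with BP_MyPlayer, death zones respawn the player and checkpoints set a new spawn from the Arrow's world location and rotation at unit scale.
; Win zones pause the game, show WBP_EndScreen and switch to UI-only input with a visible cursor.
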(event `self.Box.OnComponentBeginOverlap`
  (params (OverlappedComponent :type "PrimitiveComponent Object Reference") (OtherActor :type "Actor Object Reference") (OtherComp :type "PrimitiveComponent Object Reference") (OtherBodyIndex :type Integer) (bFromSweep :type Boolean) (SweepResult :type "HitResult Structure (by ref)"))
  (bind _returnvalue (`GameplayStatics.GetPlayerController` 0))
  (bind _endscreenwidget (`self.EndScreenWidget`))
  (bind (_returnvalue_location _returnvalue_rotation) (`KismetMathLibrary.BreakTransform` (`SceneComponent.K2_GetComponentToWorld` (`self.Arrow`))))
  (bind _asbp_my_player (cast `/Game/Asset/Characters/BP_MyPlayer` OtherActor))
  (switch `/Game/Asset/TriggerBoxes/E_TriggerZone` (`self.ZoneType`)
    (:`NewEnumerator0`
      (`/Game/Asset/Characters/BP_MyPlayer.Respawn` _asbp_my_player))
    (:`NewEnumerator1`
      (`/Game/Asset/Characters/BP_MyPlayer.SetNewSpawnTransform` _asbp_my_player (`KismetMathLibrary.MakeTransform` _returnvalue_location _returnvalue_rotation)))
    (:`NewEnumerator2`
      (`GameplayStatics.SetGamePaused` true)
      (bind _returnvalue_2 (`|CreateWidget` "/Game/Asset/Widgets/WBP_EndScreen.WBP_EndScreen_C"))
      (set `self.EndScreenWidget` _returnvalue_2)
      (`UserWidget.AddToViewport` _endscreenwidget 0)
      (`WidgetBlueprintLibrary.SetInputMode_UIOnlyEx` _returnvalue _endscreenwidget)
      (set `PlayerController.bShowMouseCursor` true _returnvalue))))

(fn `UserConstructionScript`)