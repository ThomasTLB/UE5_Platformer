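; Moving platform actor that shuttles endlessly between the StartMesh and EndMesh markers from BeginPlay.
; The Moving timeline lerps the platform's world transform between both markers without sweep, at a play rate inverted from PlayRate so larger values move slower.
; On finish it stores the timeline direction and calls MovingEvent again to play the opposite way.
; The construction script shows the markers in red or hides them with an invisible material via ShowStartEndMesh.
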(event `self.ReceiveBeginPlay`
  (`self.Moving Event`))

(event `Moving Event`
  (`TimelineComponent.SetPlayRate` (`self.Moving`) (/ 1.0 (`self.PlayRate`)))
  (switch `ETimelineDirection` (`self.Direction`)
    (:`Forward`
      (bind (_direction _moving) (`Timeline|Moving` :!via `ReverseFromEnd` :!label _label)
        (:`Update`
          (`SceneComponent.K2_SetWorldTransform` (`self.Platform`) (`KismetMathLibrary.TLerp` (`SceneComponent.K2_GetComponentToWorld` (`self.StartMesh`)) (`SceneComponent.K2_GetComponentToWorld` (`self.EndMesh`)) _moving) false false))
        (:`Finished`
          (set `self.Direction` _direction)
          (`self.Moving Event`))))
    (:`Backward`
      (goto _label :!via `PlayFromStart`))))

(fn `UserConstructionScript`
  (if (`self.ShowStartEndMesh`)
    (`PrimitiveComponent.SetMaterial` (`self.EndMesh`) 0 "/Game/Asset/Material/M_RedMesh.M_RedMesh")
    (`PrimitiveComponent.SetMaterial` (`self.StartMesh`) 0 "/Game/Asset/Material/M_RedMesh.M_RedMesh")
    (else
      (`PrimitiveComponent.SetMaterial` (`self.StartMesh`) 0 "/Game/Asset/Material/M_Invis.M_Invis")
      (`PrimitiveComponent.SetMaterial` (`self.EndMesh`) 0 "/Game/Asset/Material/M_Invis.M_Invis"))))