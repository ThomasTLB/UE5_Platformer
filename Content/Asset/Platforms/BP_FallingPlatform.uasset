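; Falling platform that wobbles or tilts when the player character enters its trigger box, then drops.
; A one-shot overlap starts the Rotate timeline, which drives the cube's world roll, then enables physics simulation when it finishes.
; A Respawn event teleports the cube back to its BeginPlay transform and re-arms it after a delay, which a FastRespawn flag can skip.
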(event `self.ReceiveBeginPlay`
  (set `self.defaultSpawn` (`SceneComponent.K2_GetComponentToWorld` (`self.Cube`))))

(event `self.Box.OnComponentBeginOverlap`
  (params (OverlappedComponent :type "PrimitiveComponent Object Reference") (OtherActor :type "Actor Object Reference") (OtherComp :type "PrimitiveComponent Object Reference") (OtherBodyIndex :type Integer) (bFromSweep :type Boolean) (SweepResult :type "HitResult Structure (by ref)"))
  (if (and (== OtherActor (`GameplayStatics.GetPlayerCharacter` 0)) (`self.CanBePlayed?`))
    (set `self.CanBePlayed?` false)
    (bind (_direction _rotatevalue) (`Timeline|Rotate` :!via `PlayFromStart`)
      (:`Update`
        (`SceneComponent.K2_SetWorldRotation` (`self.Cube`) (`KismetMathLibrary.MakeRotator` _rotatevalue) false false))
      (:`Finished`
        (`PrimitiveComponent.SetSimulatePhysics` (`self.Cube`) true)
        (`self.Respawn` false)))))

(event `Respawn`
  (params (`fastRespawn?` :type Boolean))
  (if (not `fastRespawn?`)
    (`KismetSystemLibrary.Delay` 5.0))
  (`PrimitiveComponent.SetSimulatePhysics` (`self.Cube`) false)
  (`SceneComponent.K2_SetWorldTransform` (`self.Cube`) (`self.defaultSpawn`) false true)
  (set `self.CanBePlayed?` true))

(fn `UserConstructionScript`)