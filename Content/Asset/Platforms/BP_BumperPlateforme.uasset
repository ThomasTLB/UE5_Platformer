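; Bumper platform that launches BP_MyPlayer when the player overlaps its Box trigger.
; The launch always applies a vertical velocity and adds a push along the direction arrow when LaunchForward is enabled.
; The launch adds to the player's current velocity rather than overriding it.
; The construction script shows the arrow component only when LaunchForward is on, as a preview of the launch direction.
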(event `self.ReceiveBeginPlay`)

(event `self.Box.OnComponentBeginOverlap`
  (params (OverlappedComponent :type "PrimitiveComponent Object Reference") (OtherActor :type "Actor Object Reference") (OtherComp :type "PrimitiveComponent Object Reference") (OtherBodyIndex :type Integer) (bFromSweep :type Boolean) (SweepResult :type "HitResult Structure (by ref)"))
  (bind _asbp_my_player (cast `/Game/Asset/Characters/BP_MyPlayer` OtherActor))
  (`Character.LaunchCharacter` _asbp_my_player (+ (* (`SceneComponent.GetForwardVector` (`self.LanchDirectionArrow`)) (`KismetMathLibrary.SelectFloat` (`self.LaunchVelocityX`) 0.0 (`self.bLaunchForward`))) (`KismetMathLibrary.MakeVector` 0.0 0.0 (`self.LaunchVelocityZ`))) false false))

(event `UpdateArrowVisibility`
  (`SceneComponent.SetVisibility` (`self.LanchDirectionArrow`) (`self.bLaunchForward`) false))

(fn `UserConstructionScript`
  (`self.UpdateArrowVisibility`))